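; Enemy security camera that turns toward and shoots a target entering its detection sphere, and dies from any damage.
; The sphere overlap enables Tick, which requires every ConditionRequirementComponent found at construction to pass before turning the spotlights red and rotating via FaceTarget.
; Shooter fires once a dot-product check shows the player within aiming tolerance.
; Damage notifies ScoreByDamageGameMode, plays explosion effects and destroys the actor.
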(event `self.ReceiveTick`
  (params (DeltaSeconds :type "Float (single-precision)"))
  ;[1 1 1] Tracking and shooting
  (bind _bmet (`self.CheckConditions`))
  (if _bmet
    (`LightComponent.SetLightColor` (`self.SpotLight`) (struct :`R` 1.0 :`A` 1.0) true)
    (`LightComponent.SetLightColor` (`self.SpotLight1`) (struct :`R` 1.0 :`A` 1.0) true)
    (if (not (`FaceTargetComponent.IsRotating` (`self.FaceTarget`)))
      (`FaceTargetComponent.StartRotating` (`self.FaceTarget`) (`self.TargetActor`)))
    (if (`self.IsFacingPlayer`)
      (`ShooterComponent.Shoot` (`self.Shooter`)))
    (else
      (`LightComponent.SetLightColor` (`self.SpotLight`) (struct :`B` 1.0 :`A` 1.0) true)
      (`LightComponent.SetLightColor` (`self.SpotLight1`) (struct :`B` 1.0 :`A` 1.0) true)
      (`FaceTargetComponent.StopRotating` (`self.FaceTarget`)))))

(event `self.Sphere.OnComponentBeginOverlap`
  (params (OverlappedComponent :type "PrimitiveComponent Object Reference") (OtherActor :type "Actor Object Reference") (OtherComp :type "PrimitiveComponent Object Reference") (OtherBodyIndex :type Integer) (bFromSweep :type Boolean) (SweepResult :type "HitResult Structure (by ref)"))
  ;[1 1 1] Actor Enters/leaves range
  (set `self.TargetActor` OtherActor)
  (`self.SetActorTickEnabled` true))

(event `self.Sphere.OnComponentEndOverlap`
  (params (OverlappedComponent :type "PrimitiveComponent Object Reference") (OtherActor :type "Actor Object Reference") (OtherComp :type "PrimitiveComponent Object Reference") (OtherBodyIndex :type Integer))
  ;[1 1 1] Actor Enters/leaves range
  (`self.SetActorTickEnabled` false)
  (set `self.TargetActor` null))

(event `self.ReceiveAnyDamage`
  (params (Damage :type "Float (single-precision)") (DamageType :type "DamageType Object Reference") (InstigatedBy :type "Controller Object Reference") (DamageCauser :type "Actor Object Reference"))
  ;[1 1 1] Death
  (`self.SetActorTickEnabled` false)
  (`SceneComponent.SetVisibility` (`self.StaticMesh`) false false)
  (`PrimitiveComponent.SetCollisionEnabled` (`self.Sphere`) "NoCollision")
  (bind _asscore_by_damage_game_mode (cast `ScoreByDamageGameMode` (`GameplayStatics.GetGameMode`))
    (:`then`
      (`ScoreByDamageGameMode.EnemyDestroyed` _asscore_by_damage_game_mode DamageType))
    (:`CastFailed`
      _))
  (`GameplayStatics.SpawnEmitterAtLocation` "/Game/StarterContent/Particles/P_Explosion.P_Explosion" (`self.K2_GetActorLocation`))
  (`GameplayStatics.PlaySound2D` "/Game/StarterContent/Audio/Explosion01.Explosion01" 1.0 1.0 0.0 null null)
  (`self.K2_DestroyActor`))

(fn `CheckConditions`
  (returns (bMet :type Boolean))
  (for _array_element (`self.Conditions`)
    (if (not (`ConditionRequirementComponent.IsConditionMet` _array_element (`self.TargetActor`)))
      (return false)))
  (return true))

(fn `IsFacingPlayer`
  (returns (bFacingPlayer :type Boolean))
  (return (`KismetMathLibrary.InRange_FloatFloat` (`KismetMathLibrary.Dot_VectorVector` (`self.GetActorForwardVector`) (`KismetMathLibrary.GetForwardVector` (`KismetMathLibrary.FindLookAtRotation` (`self.K2_GetActorLocation`) (`self.K2_GetActorLocation` (`GameplayStatics.GetPlayerCharacter` 0))))) (- 1.0 (`self.AimingTolerance`)) 1.1)))

(fn `UserConstructionScript`
  (set `self.Conditions` (`self.K2_GetComponentsByClass` "/Script/FueroTask.ConditionRequirementComponent")) ; Collecting all of the required conditions
  (`SphereComponent.SetSphereRadius` (`self.Sphere`) (`self.In Sphere Radius`) true)
  (set `ShooterComponent.ShotOriginOffset` (`self.ShootingPoint`) (`self.Shooter`)))