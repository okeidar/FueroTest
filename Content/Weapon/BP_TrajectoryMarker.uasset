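; Trajectory marker that draws a projected path as a Niagara beam following a spline.
; UpdateTrajectoryPoint resizes the spline to the supplied points, sets them in world space as linear points, then prepends the owner's location as the origin.
; Spline edits are batched into a single update, and the beam shows only when the point count exceeds a minimum.
; SetTrajectoryVisible toggles the beam's activation and visibility.
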(event `self.ReceiveBeginPlay`
  (`SplineComponent.ClearSplinePoints` (`self.Spline`) true))

(fn `AddLocationsToSpline`
  (params (Locations :type "Array of Vector Structure"))
  (for (_array_element _array_index) Locations
    (`SplineComponent.SetLocationAtSplinePoint` (`self.Spline`) _array_index _array_element "World" false)
    (`SplineComponent.SetSplinePointType` (`self.Spline`) _array_index "Linear" false))
  (`SplineComponent.AddSplinePointAtIndex` (`self.Spline`) (`self.K2_GetActorLocation` (`self.GetOwner`)) 0 "World" false) ; The origin location
  (`SplineComponent.SetSplinePointType` (`self.Spline`) 0 "Linear" false))

(fn `AddSplinePoints`
  (params (LastIndex :type Integer))
  (for _ (range 1 (+ LastIndex 1))
    (`SplineComponent.AddSplinePoint` (`self.Spline`) (0.0 0.0 0.0) "World" false))
  (return))

(fn `RemoveSplinePoints`
  (params (FirstIndex :type Integer))
  (for _ (range FirstIndex 0)
    (`SplineComponent.RemoveSplinePoint` (`self.Spline`) 0 false))
  (return))

(fn `SetTrajectoryVisible`
  (params (bVisible :type Boolean))
  (bind _ns_splinefollowingbeam (`self.NS_SplineFollowingBeam`))
  (`ActorComponent.SetActive` _ns_splinefollowingbeam (`local.bVisible`) true)
  (`SceneComponent.SetVisibility` _ns_splinefollowingbeam (`local.bVisible`) false)
  (return))

(fn `UpdateTrajectoryPoint`
  (params (TrajectoryPoints :type "Array of Vector Structure (by ref)"))
  (locals (SplinePointsDelta :type Integer))
  (bind _splinepointsdelta (`local.SplinePointsDelta`))
  (set `local.SplinePointsDelta` (- (`KismetArrayLibrary.Array_Length` TrajectoryPoints) (`SplineComponent.GetNumberOfSplinePoints` (`self.Spline`))))
  (`|ExecutionSequence`
    (:`then_0`
      (if (> (`local.SplinePointsDelta`) 0)
        (`self.AddSplinePoints` _splinepointsdelta)
        (elif (< (`local.SplinePointsDelta`) 0)
          (`self.RemoveSplinePoints` _splinepointsdelta))))
    (:`then_1`
      (`self.AddLocationsToSpline` (`local.TrajectoryPoints`))
      (`SplineComponent.UpdateSpline` (`self.Spline`))
      (`SceneComponent.SetVisibility` (`self.NS_SplineFollowingBeam`) (> (`KismetArrayLibrary.Array_Length` (`local.TrajectoryPoints`)) (`self.MinimumPointToShow`)) false)
      (return))))

(fn `UserConstructionScript`)