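; Weapon mode for bouncing projectiles that previews the trajectory while fire is held and launches on release.
; Fire start spawns a hidden, collisionless projectile and caches its radius, speed, gravity and lifespan.
; Tick loops path prediction from the camera aim, reflecting off surfaces until an enemy hit, miss or bounce limit, feeding points to BP_TrajectoryMarker.
; Fire end restores and launches that same projectile.
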(event `self.ReceiveBeginPlay`
  (bind _returnvalue (`|SpawnActorFromClass` "/Game/Weapon/BP_TrajectoryMarker.BP_TrajectoryMarker_C" (`KismetMathLibrary.MakeTransform` (0.0 0.0 0.0)) "Undefined" "OverrideRootScale" (`self.GetOwner`) null))
  (set `self.TrajectoryVisualizer` _returnvalue))

(event `self.ReceiveTick`
  (params (DeltaSeconds :type "Float (single-precision)"))
  ;[1 1 1] Trajectory Calcualtion
  (`|ExecutionSequence`
    (:`then_0`
      (`self.SetupInitialValues`)
      (bind (_outhit _outpathpositions _outlasttracedestination _returnvalue) (`GameplayStatics.Blueprint_PredictProjectilePath_ByTraceChannel` (`self.StartingLocation`) (`self.Velocity`) true (`self.ProjectileRadius`) "ECC_WorldDynamic" false (`|MakeArray` (`self.GetOwner`) (`self.LastHitActor`) (`GameplayStatics.GetPlayerCharacter` 0) :!type "Actor Object Reference") "None" 10.0 30.0 (`self.ProjectileLifeSpan`) (`self.ProjectileGravity`) :!label _label)) ; Whenever we keep hitting or untill we hit an enemy or we reached our max bounces
      (if _returnvalue
        (bind (_bblockinghit _binitialoverlap _time _distance _location _impactpoint _normal _impactnormal _physmat _hitactor _hitcomponent) (`GameplayStatics.BreakHitResult` _outhit))
        (if (`|EnumEquality` (`PrimitiveComponent.GetCollisionObjectType` _hitcomponent) "ECC_GameTraceChannel2")
          (`KismetArrayLibrary.Array_Add` (`self.HitLocations`) _outlasttracedestination) ; Saves enemy hit as a trajectory point and leaves
          (else
            (`/Engine/EditorBlueprintResources/StandardMacros.IncrementInt` (`self.CurrentBounceCount`)
              (:`  `
                (bind _output_get (set `self.StartingLocation` (`|GetArrayItem` _outpathpositions (`KismetArrayLibrary.Array_LastIndex` _outpathpositions))))
                (`KismetArrayLibrary.Array_Add` (`self.HitLocations`) _output_get)
                (set `self.LastHitActor` _hitactor)
                (set `self.Velocity` (`KismetMathLibrary.GetReflectionVector` (`self.Velocity`) _normal))
                (if (<= (`self.CurrentBounceCount`) (`self.MaxBounceCount`))
                  (goto _label))))))
        (else
          (`KismetArrayLibrary.Array_Add` (`self.HitLocations`) _outlasttracedestination) ; Save a point as last even if we dont hit so we can draw it
        )))
    (:`then_1`
      (`/Game/Weapon/BP_TrajectoryMarker.UpdateTrajectoryPoint` (`self.TrajectoryVisualizer`) (`self.HitLocations`)))))

(event `self.BeginFire`
  ;[1 1 1] Shooting
  (`self.SpawnProjectileAndCacheDefaults`)
  (`self.SetComponentTickEnabled` true)
  (`/Game/Weapon/BP_TrajectoryMarker.SetTrajectoryVisible` (`self.TrajectoryVisualizer`) true))

(event `self.EndFire`
  ;[1 1 1] Shooting
  (`self.SetComponentTickEnabled` false)
  (`self.Release Projectile`)
  (`/Game/Weapon/BP_TrajectoryMarker.SetTrajectoryVisible` (`self.TrajectoryVisualizer`) false))

(fn `Release Projectile`
  (bind _projectilemovement (`BaseProjectile.ProjectileMovement` (`self.SpawnedProjectile`)))
  (bind _returnvalue (`PlayerCameraManager.GetCameraRotation` (`PlayerController.PlayerCameraManager` (`GameplayStatics.GetPlayerController` 0))))
  (`/Engine/EditorBlueprintResources/StandardMacros.IsValid` (`self.SpawnedProjectile`)
    (:`Is Valid`
      (`Actor.K2_SetActorLocation` (`self.SpawnedProjectile`) (`Actor.K2_GetActorLocation` (`self.GetOwner`)) false false)
      (`Actor.SetLifeSpan` (`self.SpawnedProjectile`) (`self.ProjectileLifeSpan`))
      (`PrimitiveComponent.SetCollisionEnabled` (`BaseProjectile.CollisionComponent` (`self.SpawnedProjectile`)) "QueryAndPhysics")
      (`Actor.SetActorHiddenInGame` (`self.SpawnedProjectile`) false)
      (set `MovementComponent.Velocity` (`KismetMathLibrary.GreaterGreater_VectorRotator` (* (`self.InitialSpeed`) (1.0 0.0 0.0)) (`KismetMathLibrary.ComposeRotators` _returnvalue (`KismetMathLibrary.RotatorFromAxisAndAngle` (`KismetMathLibrary.GetRightVector` _returnvalue) (`self.CameraAimUpOffsetDegrees`)))) _projectilemovement)
      (`self.Activate` _projectilemovement false)
      (set `self.SpawnedProjectile` null)
      (return))))

(fn `SpawnProjectileAndCacheDefaults`
  (bind _spawnedprojectile (`self.SpawnedProjectile`))
  (bind _projectilemovement (`BaseProjectile.ProjectileMovement` (`self.SpawnedProjectile`)))
  (bind _collisioncomponent (`BaseProjectile.CollisionComponent` (`self.SpawnedProjectile`)))
  (bind _returnvalue (`|SpawnActorFromClass` (`self.ProjectileClass`) (`KismetMathLibrary.MakeTransform` (0.0 0.0 0.0)) "Undefined" "OverrideRootScale" null null))
  (set `self.SpawnedProjectile` _returnvalue)
  (`|ExecutionSequence`
    (:`then_0`
      (set `self.ProjectileLifeSpan` (`Actor.GetLifeSpan` _spawnedprojectile))
      (`Actor.SetLifeSpan` _spawnedprojectile 0.0))
    (:`then_1`
      (`Actor.SetActorHiddenInGame` (`self.SpawnedProjectile`) true))
    (:`then_2`
      (`PrimitiveComponent.SetCollisionEnabled` _collisioncomponent "NoCollision")
      (set `self.ProjectileRadius` (`SphereComponent.SphereRadius` _collisioncomponent)))
    (:`then_3`
      (set `self.InitialSpeed` (`ProjectileMovementComponent.InitialSpeed` _projectilemovement))
      (set `self.ProjectileGravity` (+ (`MovementComponent.GetGravityZ` _projectilemovement) 0.0001)))
    (:`then_4`
      (return))))