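; Weapon actor that delegates firing to a third-person or first-person weapon mode, swapped when the point of view changes.
; Begin and end fire are forwarded to the active mode, while the construction script passes shot origin to both and the aim offset to the third-person one.
; Each tick, a trace from the weapon along camera direction, pitched by that offset in third person, sets the laser effect's endpoint.
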(event `self.ReceiveBeginPlay`
  (set `self.ActiveWeapon` (`self.ThirdPersonWeaponMode`))
  (set `self.AimIgnore` (`|MakeArray` (`self.GetOwner`) self :!type "Actor Object Reference")))

(event `self.SwitchMode`
  (params (NewMode :type "ESupportedModes Enum" :default "ESM_TPS"))
  ;[1 1 1] Mode Switch
  (bind _output_get (set `self.CurrentPOV` NewMode))
  (switch `ESupportedModes` _output_get
    (:`ESM_TPS`
      (set `self.ActiveWeapon` (`self.ThirdPersonWeaponMode`)))
    (:`ESM_FPS`
      (set `self.ActiveWeapon` (`self.FirstPersonWeaponMode`)))))

(event `self.BeginFire`
  ;[1 1 1] Shooting
  (message `CanFire.BeginFire` (`self.ActiveWeapon`)))

(event `self.EndFire`
  ;[1 1 1] Shooting
  (message `CanFire.EndFire` (`self.ActiveWeapon`)))

(event `self.ReceiveTick`
  (params (DeltaSeconds :type "Float (single-precision)"))
  (bind _returnvalue (`self.K2_GetActorLocation`))
  (bind _returnvalue_2 (`PlayerCameraManager.GetCameraRotation` (`GameplayStatics.GetPlayerCameraManager` 0)))
  (bind _returnvalue_3 (+ _returnvalue (`KismetMathLibrary.GreaterGreater_VectorRotator` (* (`KismetMathLibrary.GetForwardVector` _returnvalue_2) 5000.0) (`KismetMathLibrary.RotatorFromAxisAndAngle` (`KismetMathLibrary.GetRightVector` _returnvalue_2) (select `ESupportedModes` (`self.CurrentPOV`) :`ESM_TPS` (`self.CameraAimUpOffsetDegrees`) :!type "Float (single-precision)")))))
  (bind (_outhit _returnvalue_4) (`KismetSystemLibrary.LineTraceSingle` _returnvalue _returnvalue_3 "TraceTypeQuery1" false (`self.AimIgnore`)))
  (if _returnvalue_4
    (`FXSystemComponent.SetVectorParameter` (`self.LaserFX`) "LaserEnd" (`.ImpactPoint` (`GameplayStatics.BreakHitResult` _outhit)))
    (else
      (`FXSystemComponent.SetVectorParameter` (`self.LaserFX`) "LaserEnd" _returnvalue_3))))

(fn `UserConstructionScript`
  (bind _shotorigin (`self.ShotOrigin`))
  (set `WeaponMode.ShotOriginOffset` _shotorigin (`self.ThirdPersonWeaponMode`))
  (set `WeaponMode.ShotOriginOffset` _shotorigin (`self.FirstPersonWeaponMode`))
  (set `/Game/Weapon/BP_BouncyWeaponMode.CameraAimUpOffsetDegrees` (`self.CameraAimUpOffsetDegrees`) (`self.ThirdPersonWeaponMode`)))