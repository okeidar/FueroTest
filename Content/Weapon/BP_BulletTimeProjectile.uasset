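; BP_BulletTimeProjectile is a projectile that triggers a slow-motion bullet-cam while it exists.
; On BeginPlay it disables input, blends the player's view to itself, hides the character and sets global time dilation to slow motion.
; On hit it runs the parent logic, hides itself and spawns a small explosion.
; Time, view, character visibility and input are restored only when the actor is destroyed.
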(event `self.ReceiveBeginPlay`
  (bind _returnvalue (`GameplayStatics.GetPlayerController` 0))
  (`self.DisableInput` (`GameplayStatics.GetPlayerCharacter` 0) _returnvalue)
  (`self.DisableInput` _returnvalue _returnvalue)
  (`PlayerController.SetViewTargetWithBlend` _returnvalue self 0.2 "VTBlend_Linear" 0.0 false)
  (message `/Game/ThirdPerson/Blueprints/BPI_CanHide.SetCharacterHidden` (`GameplayStatics.GetPlayerCharacter` 0) true)
  (`GameplayStatics.SetGlobalTimeDilation` 0.1))

(event `self.ReceiveDestroyed`
  (bind _returnvalue (`GameplayStatics.GetPlayerCharacter` 0))
  (bind _returnvalue_2 (`GameplayStatics.GetPlayerController` 0))
  ;[1 1 1] Destroyed
  (`GameplayStatics.SetGlobalTimeDilation` 1.0)
  (`PlayerController.SetViewTargetWithBlend` _returnvalue_2 _returnvalue 0.2 "VTBlend_Linear" 0.0 false)
  (message `/Game/ThirdPerson/Blueprints/BPI_CanHide.SetCharacterHidden` _returnvalue false)
  (`self.EnableInput` _returnvalue _returnvalue_2)
  (`self.EnableInput` _returnvalue_2 _returnvalue_2))

(event `self.OnHit`
  (params (HitComp :type "PrimitiveComponent Object Reference") (OtherActor :type "Actor Object Reference") (OtherComp :type "PrimitiveComponent Object Reference") (NormalImpulse :type "Vector Structure") (Hit :type "HitResult Structure (by ref)"))
  ;[1 1 1] Hit
  (`parent.OnHit` HitComp OtherActor OtherComp NormalImpulse Hit)
  (`SceneComponent.SetVisibility` (`self.RootComponent`) false true)
  (`GameplayStatics.SpawnEmitterAtLocation` "/Game/StarterContent/Particles/P_Explosion.P_Explosion" (`self.K2_GetActorLocation`) (struct) (0.2 0.2 0.2)))

(fn `UserConstructionScript`)