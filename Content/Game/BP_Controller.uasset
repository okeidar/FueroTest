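; BP_Controller is a controller that turns player input into POV switching, shooting and zoom for the controlled pawn.
; On BeginPlay it sets the pawn's POVModeSwitcher component to third person and passes FOV zoom bounds to the pawn.
; SwitchPOV resets zoom, toggles first/third person through the switcher and swaps the matching gameplay tag, which limits zoom to first person.
; Pawn actions go through message calls, and switching POV also stops firing.
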(event `self.ReceiveBeginPlay`
  (bind _output_get (set `self.PovSwitcher` (`self.GetComponentByClass` (`self.K2_GetPawn`) "/Script/FueroTask.POVModeSwitcher")))
  (message `ModeSwitcher.SwitchMode` _output_get "ESM_TPS")
  (message `/Game/ThirdPerson/Blueprints/BPI_CanZoom.SetZoomBounds` (`self.K2_GetPawn`) (`self.MaxFOV`) (`self.Min FOV`)))

(event `InputAction|SwitchPov`
  (params (Key :type "Key Structure"))
  ;[1 1 1] POV Mode
  (:`Pressed`
    (message `CanFire.EndFire` (`self.K2_GetPawn`))
    (`self.SwitchPOV`)))

(event `InputAction|Shoot`
  (params (Key :type "Key Structure"))
  (bind _returnvalue (`self.K2_GetPawn`))
  ;[1 1 1] Shooting
  (:`Pressed`
    (message `CanFire.BeginFire` _returnvalue))
  (:`Released`
    (message `CanFire.EndFire` _returnvalue)))

(event `InputAction|ZoomIn`
  (params (Key :type "Key Structure"))
  ;[1 1 1] Zoom
  (:`Pressed`
    (if (`GameplayTagAssetInterface.HasMatchingGameplayTag` (struct :`TagName` "POVMode.FPS"))
      (message `/Game/ThirdPerson/Blueprints/BPI_CanZoom.Zoom` (`self.K2_GetPawn`) -3.0))))

(event `InputAction|ZoomOut`
  (params (Key :type "Key Structure"))
  ;[1 1 1] Zoom
  (:`Pressed`
    (if (`GameplayTagAssetInterface.HasMatchingGameplayTag` (struct :`TagName` "POVMode.FPS"))
      (message `/Game/ThirdPerson/Blueprints/BPI_CanZoom.Zoom` (`self.K2_GetPawn`) 3.0))))

(fn `SwitchPOV`
  (locals (NewTag :type "ESupportedModes Enum"))
  (bind _gameplaytags (`self.GameplayTags`))
  (message `/Game/ThirdPerson/Blueprints/BPI_CanZoom.ResetZoom` (`self.K2_GetPawn`))
  (bind _output_get (set `local.NewTag` (select `bool` (`GameplayTagAssetInterface.HasMatchingGameplayTag` (struct :`TagName` "POVMode.TPS")) :`false` "ESM_TPS" :`true` "ESM_FPS" :!type "ESupportedModes Enum")))
  (`POVModeSwitcher.SwitchModeToAllObjects` (`self.PovSwitcher`) _output_get)
  (`BlueprintGameplayTagLibrary.RemoveGameplayTag` _gameplaytags (select `ESupportedModes` (`local.NewTag`) :`ESM_TPS` (struct :`TagName` "POVMode.FPS") :`ESM_FPS` (struct :`TagName` "POVMode.TPS") :!type "GameplayTag Structure"))
  (`BlueprintGameplayTagLibrary.AddGameplayTag` _gameplaytags (select `ESupportedModes` (`local.NewTag`) :`ESM_TPS` (struct :`TagName` "POVMode.TPS") :`ESM_FPS` (struct :`TagName` "POVMode.FPS") :!type "GameplayTag Structure"))
  (return))

(fn `UserConstructionScript`)