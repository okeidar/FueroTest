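; BP_POVGameMode is the GameMode that keeps the player's score for destroyed enemies.
; Its EnemyDestroyed event checks the damage type class, awarding more points for FPS damage kills than TPS ones and none for other types.
; After each increase it broadcasts the new total through OnScoreUpdated.
; The scoring rules are hardcoded, with a note suggesting a data table for more complex rules.
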(event `self.EnemyDestroyed`
  (params (DestroyingDamage :type "DamageType Object Reference"))
  (bind _returnvalue (`GameplayStatics.GetObjectClass` DestroyingDamage))
  (if (== _returnvalue "/Game/Weapon/UFPSDamageType.UFPSDamageType_C")
    (bind _output_get (set `self.PlayerScore` (+ (`self.PlayerScore`) 5)))
    (`self.OnScoreUpdated` _output_get)
    (elif (== _returnvalue "/Game/Weapon/UTPSDamageType.UTPSDamageType_C")
      (bind _output_get_2 (set `self.PlayerScore` (+ (`self.PlayerScore`) 1)))
      (`self.OnScoreUpdated` _output_get_2))))

(fn `UserConstructionScript`)